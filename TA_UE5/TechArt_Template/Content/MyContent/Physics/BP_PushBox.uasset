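; BP_PushBox is a physics box that kicks up dust when the third-person character pushes it.
; On a component hit from that character, if the box has nonzero velocity, it spawns an attached NS_Dust Niagara system below the box and starts a short timer.
; EndSystem deactivates and destroys the most recently stored dust component, apparently as the timer's callback.
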(event OnComponentHit(Box)
  (params (HitComponent :type Primitive%20Component%20Object%20Reference) (OtherActor :type Actor%20Object%20Reference) (OtherComp :type Primitive%20Component%20Object%20Reference) (NormalImpulse :type Vector :default "0, 0, 0") (Hit :type Hit%20Result%20Structure%20%28by%20ref%29))
  (Utilities|Casting|CastToBP_ThirdPersonCharacter OtherActor)
  (if (Utilities|Operators|NotEqual(!=) :A (Transformation|GetComponentVelocity (Variables|Default|GetBox)))
    (bind _returnvalue (Niagara|SpawnSystemAttached "/Game/MyContent/FX/Dust/NS_Dust.NS_Dust" (Variables|Default|GetBox) "None" "0.000000,0.000000,-50.000000" "0, 0, 0" "KeepRelativeOffset" true))
    (Variables|Default|SetNS_System _returnvalue)
    (Utilities|Time|SetTimerbyEvent (EventDispatchers|CreateEvent :!event Custom|EndSystem) 1.0)))

(event Custom|EndSystem
  (bind _ns_system (Variables|Default|GetNS_System)
    (:then
      (Components|Activation|Deactivate _ns_system)
      (Components|DestroyComponent _ns_system))
    (:else)))

(event EventBeginPlay)

(event Collision|EventActorBeginOverlap
  (params (OtherActor :type Actor%20Object%20Reference)))

(fn ConstructionScript)