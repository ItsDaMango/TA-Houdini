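; Procedural physics rope bridge actor, built entirely in the construction script from plank count, spacing and size variables.
; It lays planks along local X with randomly alternated tilt and facing, then links neighbors with physics constraints offset by half the spacing.
; The first and last planks have physics simulation disabled to act as anchors.
; Two side cables end at the last plank's X, and pole meshes are added in pairs at both ends.
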(event EventBeginPlay)

(event Collision|EventActorBeginOverlap
  (params (OtherActor :type Actor%20Object%20Reference)))

(event EventTick
  (params (DeltaSeconds :type Float%20%28single-precision%29)))

(fn ConstructionScript
  (bind _planks (Variables|Default|GetPlanks))
  (bind _returnvalue (Utilities|Array|LastIndex _planks))
  (bind _output (Utilities|Array|Get(acopy) _planks _returnvalue))
  (bind _relativelocation (Variables|/Script/Engine.SceneComponent|GetRelativeLocation _output))
  (CallFunction|SetPlanks)
  (CallFunction|AddPlanks)
  (CallFunction|AddConstrains)
  (Physics|SetSimulatePhysics (Utilities|Array|Get(acopy) (Variables|Default|GetPlanks)) false)
  (Variables|/Script/CableComponent.CableComponent|SetEndLocation (Variables|Default|GetCable) (Math|Vector|MakeVector (.x _relativelocation) -9e+01 1e+02))
  (Variables|/Script/CableComponent.CableComponent|SetEndLocation (Variables|Default|GetCable1) (Math|Vector|MakeVector (.x _relativelocation) 9e+01 1e+02))
  (CallFunction|SpawnPoles))

(fn AddPlanks
  (for _index (range 0 (Variables|Default|GetPlankAmount))
    (bind _returnvalue (AddComponent|AddStaticMeshComponent false (Math|Transform|MakeTransform (Math|Vector|MakeVector (Math|Conversions|ToFloat(Integer) (* _index (Variables|Default|GetPlankSpacing))) 0.0 0.0) (Utilities|Select :Index (Math|Random|RandomIntegerinRange 0 1) :Option%200 "1.000000,90.000000,0.000000" :Option%201 "-1.000000,-90.000000,0.000000") (Math|Vector|MakeVector (Variables|Default|GetPlankWidth) (Variables|Default|GetPlankLength) 2.0))))
    (Utilities|Array|Add (Variables|Default|GetPlanks) _returnvalue)))

(fn AddConstrains
  (bind _planks (Variables|Default|GetPlanks))
  (for _index (range 0 (- (Variables|Default|GetPlankAmount) 1))
    (LocalVariables|SetLConstrainIndex _index)
    (bind _returnvalue (AddComponent|AddPhysicsConstraintComponent false (Math|Transform|MakeTransform (Math|Vector|MakeVector (+ (.x (Variables|/Script/Engine.SceneComponent|GetRelativeLocation (Utilities|Array|Get(acopy) (Variables|Default|GetPlanks) _index))) (Variables|Default|GetConstraintSpacing)) 0.0 0.0) "0, 0, 0" "1.000000,1.000000,1.000000")))
    (Class|PhysicsConstraintComponent|SetConstrainedComponents _returnvalue (Utilities|Array|Get(acopy) _planks (LocalVariables|GetLConstrainIndex)) "None" (Utilities|Array|Get(acopy) _planks (+ (LocalVariables|GetLConstrainIndex) 1)) "None")))

(fn SetPlanks
  (bind _output_get (Variables|Default|SetPlankSpacing (Variables|Default|GetPlankSpacing)))
  (Variables|Default|SetConstraintSpacing (Math|Conversions|ToFloat(Integer) (/ _output_get 2))))

(fn SpawnPoles
  (bind _planks (Variables|Default|GetPlanks))
  (bind _returnvalue (Utilities|Array|LastIndex _planks))
  (bind _output (Utilities|Array|Get(acopy) _planks _returnvalue))
  (bind _relativelocation (Variables|/Script/Engine.SceneComponent|GetRelativeLocation _output))
  (Utilities|FlowControl|Sequence
    (:then_0
      (AddComponent|AddStaticMeshComponent false (Math|Transform|MakeTransform "-20.000000,-90.000000,80.000000" "90.000000,90.000000,0.000000" "0.500000,0.500000,0.500000"))
      (AddComponent|AddStaticMeshComponent false (Math|Transform|MakeTransform "-20.000000,90.000000,80.000000" "90.000000,90.000000,0.000000" "0.500000,0.500000,0.500000")))
    (:then_1
      (AddComponent|AddStaticMeshComponent false (Math|Transform|MakeTransform (Math|Vector|MakeVector (.x _relativelocation) -9e+01 8e+01) "90.000000,90.000000,0.000000" "0.500000,0.500000,0.500000"))
      (AddComponent|AddStaticMeshComponent false (Math|Transform|MakeTransform (Math|Vector|MakeVector (.x _relativelocation) 9e+01 8e+01) "90.000000,90.000000,0.000000" "0.500000,0.500000,0.500000")))))